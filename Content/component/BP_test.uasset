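; BP_test is a functional test that checks where the player's ball is relative to the YPRAVLENIE pawn's cube.
; PrepareTest records the cube's world location, takes the pawn's Playerball and binds to its Callball dispatcher.
; When Callball fires, the test finishes with Default if the ball sphere's Y exceeds the recorded cube Y, otherwise Failed.
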(event `self.ReceivePrepareTest`
  (bind _asypravlenie (cast `/Game/component/YPRAVLENIE` (`GameplayStatics.GetPlayerPawn` 0)))
  (set `self.move` (`SceneComponent.K2_GetComponentLocation` (`/Game/component/YPRAVLENIE.Cube` _asypravlenie)))
  (bind _output_get (set `self.ball` (`/Game/component/YPRAVLENIE.playerball` _asypravlenie)))
  (add `/Game/component/SHERA.callball` _output_get (delegate `callball_Event_0`)))

(event `callball_Event_0`
  (bind (_move_x _move_y) (`KismetMathLibrary.BreakVector` (`self.move`)))
  (bind (_returnvalue_x _returnvalue_y) (`KismetMathLibrary.BreakVector` (`SceneComponent.K2_GetComponentLocation` (`/Game/component/SHERA.Sphere` (`self.ball`)))))
  (if (< _move_y _returnvalue_y)
    (`self.FinishTest` "Default")
    (else
      (`self.FinishTest` "Failed"))))

(fn `NewFunction_0`)

(fn `OnRep_move`)

(fn `UserConstructionScript`)